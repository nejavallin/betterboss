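; BPC_HitFlash is an actor component that briefly flashes the owner's skeletal mesh when it takes damage.
; On BeginPlay it builds a tinted dynamic material instance, and if the owner has a BPC_Health, caches the mesh and its materials and binds to damage applied.
; Each hit puts the flash material on the first two material slots, waits the flash duration, then restores the cached material list.
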(event `self.ReceiveBeginPlay`
  (bind _returnvalue (`self.GetOwner`))
  (bind _returnvalue_2 (`Actor.GetComponentByClass` _returnvalue "/Script/Engine.SkeletalMeshComponent"))
  (bind _returnvalue_3 (`Actor.GetComponentByClass` _returnvalue "/Game/Blueprints/Components/BPC_Health.BPC_Health_C"))
  (bind _returnvalue_4 (`KismetMaterialLibrary.CreateDynamicMaterialInstance` (`self.HitflashMaterial`)))
  (bind _output_get (set `self.HitflashMID` _returnvalue_4))
  (`MaterialInstanceDynamic.SetVectorParameterValue` _output_get "BaseColor" (`self.BaseColor`))
  (`MaterialInstanceDynamic.SetVectorParameterValue` _output_get "EmmesiveColor" (`self.EmmisiveColor`))
  (`/Engine/EditorBlueprintResources/StandardMacros.IsValid` _returnvalue_3
    (:`Is Valid`
      (set `self.OG_Mesh` _returnvalue_2)
      (set `self.OGMaterials` (`MeshComponent.GetMaterials` _returnvalue_2))
      (add `/Game/Blueprints/Components/BPC_Health.OnDamageApplied` _returnvalue_3 (delegate `HitFlash`)))))

(event `HitFlash`
  (bind _hitflashmid (`self.HitflashMID`))
  (bind _og_mesh (`self.OG_Mesh`))
  (`PrimitiveComponent.SetMaterial` _og_mesh 0 _hitflashmid)
  (`PrimitiveComponent.SetMaterial` _og_mesh 1 _hitflashmid)
  (`KismetSystemLibrary.Delay` (`self.FlashDuration`))
  (`GeometryScriptLibrary_SceneUtilityFunctions.SetComponentMaterialList` (`self.OG_Mesh`) (`self.OGMaterials`)))