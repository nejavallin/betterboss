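; Boss enemy that fights the player through three health-driven phases, with a health bar and data-table ability stats.
; Unless a State Tree is enabled, a looping timer, retimed each phase, picks artillery, cone or spinning-beam attacks by range, cooldown and phase.
; Attacks mostly spawn as ability actors, with IsBusy gating selection and player-facing rotation.
; Add summons lead to sacrifices and an apocalypse pillar used by the blast; phase three spawns a bigger enemy.
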(event `TriggerArtillery`
  ;[0.15 0.08828 0.08828 0.5 25] Artillery Attack
  (bind _returnvalue (`|SpawnActorFromClass` "/Game/Blueprints/Abilities/AB_Ability_ArtilleryStrike.AB_Ability_ArtilleryStrike_C" (`self.GetTransform`) "Undefined" "MultiplyWithRoot" null self null :!label _label))
  (add `self.OnDestroyed` _returnvalue (`|CreateDelegate` :!event `CustomEvent`)))

(event `TriggerApocalypseBlast`
  ;[0.15 0.03828 0.03828 0.5 25] Apocolypse Blast Attack
  (if (`self.IsBusy`)
    (`KismetSystemLibrary.K2_SetTimerDelegate` (`|CreateDelegate` :!event `TriggerApocalypseBlast`) 1.0)
    (else
      (set `self.IsBusy` true)
      (set `self.IsSpinning` false)
      (`/Engine/EditorBlueprintResources/StandardMacros.IsValid` (`self.ActiveBeam`)
        (:`Is Valid`
          (`self.K2_DestroyActor` (`self.ActiveBeam`)))
        (:`Is Not Valid`
          _))
      (`|SpawnActorFromClass` "/Game/Blueprints/Abilities/AB_Ability_ApocalypseBlast.AB_Ability_ApocalypseBlast_C" (`self.GetTransform`) "Undefined" "MultiplyWithRoot" null self (`self.ActivePillar`) null))))

(event `TriggerConeAttack`
  ;[0.15 0.08828 0.08828 0.5 25] Cone Attack
  (bind _returnvalue (`|SpawnActorFromClass` "/Game/Blueprints/Abilities/AB_Ability_ConeAttack.AB_Ability_ConeAttack_C" (`self.GetTransform`) "Undefined" "MultiplyWithRoot" null self null))
  (add `self.OnDestroyed` _returnvalue (delegate `CustomEvent`)))

(event `CustomEvent` :!signature `self.OnDestroyed`
  (params (DestroyedActor :type "Actor Object Reference"))
  ;[0.15 0.08828 0.08828 0.5 25] Cone Attack
  (`self.TaskComplete`))

(event `ResetArtilleryCooldown`
  ;[0.15 0.08828 0.08828 0.5 25] Artillery Attack
  (set `self.bCanCastArtillery` true))

(event `ResetBeamCooldown`
  ;[0.15 0.08828 0.08828 0.5 25] Artillery Attack
  (set `self.bCanCastBeam` true))

(event `ChooseAbility`
  (bind (_value _returnvalue) (`BlueprintMapLibrary.Map_Find` (`self.Abilities`) "NewEnumerator1"))
  (if (`self.UseStateTree`)
    _
    (elif (not (`self.IsBusy`))
      (set `self.IsBusy` true)
      (if (and (`self.bCanCastArtillery`) (> (`self.GetDistanceTo` (`self.PlayerRef`)) (`KismetMathLibrary.SelectFloat` (`.MinRange_8_2D6955FE43F088D8637C71B0671689ED` (break `/Game/Blueprints/F_AbiltyStruct` _value)) 900.0 _returnvalue)))
        (set `self.bCanCastArtillery` false)
        (`KismetSystemLibrary.K2_SetTimerDelegate` (`|CreateDelegate` :!event `ResetArtilleryCooldown`) (`self.ArtilleryCooldown`))
        (goto _label)
        (else
          (`/Engine/EditorBlueprintResources/StandardMacros.IsValid` (`self.PlayerRef`)
            (:`Is Valid`
              _)
            (:`Is Not Valid`
              (bind _asbp_player_char (cast `/Game/Blueprints/Player/BP_PlayerChar` (`GameplayStatics.GetPlayerCharacter` 0)))
              (set `self.PlayerRef` _asbp_player_char)))
          (switch `/Game/Blueprints/E_BossPhase` (`self.CurrentPhase`)
            (:`NewEnumerator0`
              (`self.TriggerConeAttack`))
            (:`NewEnumerator1`
              (if (`self.bCanCastBeam`) :!label _label_2
                (set `self.bCanCastBeam` false)
                (`KismetSystemLibrary.K2_SetTimerDelegate` (`|CreateDelegate` :!event `ResetBeamCooldown`) 35.0)
                (`self.TriggerSpinBeam`)
                (else
                  (`self.TriggerConeAttack`))))
            (:`NewEnumerator2`
              (goto _label_2))))))))

(event `self.ReceiveBeginPlay`
  ;[0.07684 0.3802 0.07272 0.5 34] BEGIN PLAY
  (`|ExecutionSequence`
    (:`then_0`
      ;; Connection to Ability Data Table
      (bind _outrownames (`DataTableFunctionLibrary.GetDataTableRowNames` "/Game/Blueprints/DT_Abilties.DT_Abilties"))
      (for _array_element _outrownames
        (bind _returnvalue (`|GetDataTableRow` "/Game/Blueprints/DT_Abilties.DT_Abilties" _array_element)
          (:`then`
            (`BlueprintMapLibrary.Map_Add` (`self.Abilities`) (`.AbilityID_21_DDB806474F3B78599912ACBC892315A1` (break `/Game/Blueprints/F_AbiltyStruct` _returnvalue)) _returnvalue))))
      ; HealthBar
      (bind _returnvalue_2 (`|CreateWidget` "/Game/UI/WBP_BossHealthBar.WBP_BossHealthBar_C" (`GameplayStatics.GetPlayerController` 0)))
      (bind _output_get (set `self.BossHealthBar` _returnvalue_2))
      (`UserWidget.AddToViewport` _output_get 0)
      (add `/Game/Blueprints/BPC_Health.OnHealthUpdated` (`self.BPC_Health`) (delegate `BossUpdateHealthBar`))
      (add `/Game/Blueprints/BPC_Health.OnDeath` (`self.BPC_Health`) (delegate `OnBossDeath`))
      (bind _asbp_player_char (cast `/Game/Blueprints/Player/BP_PlayerChar` (`GameplayStatics.GetPlayerCharacter` 0)))
      (set `self.PlayerRef` _asbp_player_char)
      (`KismetSystemLibrary.K2_SetTimerDelegate` (`|CreateDelegate` :!event `TriggerSummonAdds`) 2.0)
      ; Toggle Select Ability based on state tree
      (if (not (`self.UseStateTree`))
        (bind _returnvalue_3 (`KismetSystemLibrary.K2_SetTimerDelegate` (`|CreateDelegate` :!event `ChooseAbility`) (`self.AbilityCooldown`) true))
        (set `self.AbilityCooldownTimer` _returnvalue_3)))))

(event `BossUpdateHealthBar`
  (params (NewHealth :type "Float (double-precision) (by ref)"))
  (bind _bpc_health (`self.BPC_Health`))
  (bind _returnvalue (/ (`/Game/Blueprints/BPC_Health.Health` _bpc_health) (`/Game/Blueprints/BPC_Health.MaxHealth` _bpc_health)))
  ; HealthBar
  (`/Game/UI/WBP_BossHealthBar.Boss Set Life Percentage` (`self.BossHealthBar`) _returnvalue)
  ;[0.03903 0.1093 0.15 0.5] Phase/Stage Management
  (if (and (<= _returnvalue (`self.Phase2_TriggerThreshold`)) (`|EnumEquality` (`self.CurrentPhase`) "NewEnumerator0"))
    (set `self.CurrentPhase` "NewEnumerator1")
    (`KismetSystemLibrary.K2_ClearAndInvalidateTimerHandle` (`self.AbilityCooldownTimer`))
    (bind _returnvalue_2 (`KismetSystemLibrary.K2_SetTimerDelegate` (`|CreateDelegate` :!event `ChooseAbility`) (`self.AbilityCooldownPhase2`) true))
    (set `self.AbilityCooldownTimer` _returnvalue_2)
    (`KismetSystemLibrary.K2_SetTimerDelegate` (`|CreateDelegate` :!event `TriggerSummonAdds`) 3.0)
    (elif (and (<= _returnvalue (`self.Phase3_TriggerThreshold`)) (`|EnumEquality` (`self.CurrentPhase`) "NewEnumerator1"))
      (set `self.CurrentPhase` "NewEnumerator2")
      (bind _returnvalue_3 (`|SpawnActorFromClass` "/Game/Blueprints/AI/BP_Enemy_BiggerGuy.BP_Enemy_BiggerGuy_C" (`KismetMathLibrary.MakeTransform` (+ (`self.K2_GetActorLocation`) (* (`self.GetActorForwardVector`) -2000.0))) "Undefined" "MultiplyWithRoot" null null))
      (`KismetSystemLibrary.K2_ClearAndInvalidateTimerHandle` (`self.AbilityCooldownTimer`))
      (bind _returnvalue_4 (`KismetSystemLibrary.K2_SetTimerDelegate` (`|CreateDelegate` :!event `ChooseAbility`) (`self.AbilityCooldownPhase3`) true))
      (set `self.AbilityCooldownTimer` _returnvalue_4)
      (`KismetSystemLibrary.K2_SetTimerDelegate` (`|CreateDelegate` :!event `TriggerSummonAdds`) 10.0))))

(event `OnBossDeath`
  ; HealthBar
  (`Widget.RemoveFromParent` (`self.BossHealthBar`)))

(event `TriggerSummonAdds`
  (bind (_returnvalue_x _returnvalue_y) (`KismetMathLibrary.BreakVector` (`KismetMathLibrary.RandomUnitVector`)))
  ; spawn adds
  (set `self.IsBusy` true)
  (`NiagaraFunctionLibrary.SpawnSystemAtLocation` "/Game/VFX/Mixed_Magic_VFX_Pack/VFX/NS_Dark_Owner_Cast_Spell.NS_Dark_Owner_Cast_Spell" (`self.K2_GetActorLocation`))
  (`KismetSystemLibrary.Delay` 2.0)
  (set `self.IsBusy` false)
  (for _ (range 6)
    (`|SpawnActorFromClass` "/Game/Blueprints/AI/BP_Enemy_LilGuy.BP_Enemy_LilGuy_C" (`KismetMathLibrary.MakeTransform` (+ (* (`KismetMathLibrary.MakeVector` _returnvalue_x _returnvalue_y) 5000.0) (`self.K2_GetActorLocation`))) "Undefined" "MultiplyWithRoot" null null)
    (`self.SpawnDefaultController`))
  (`KismetSystemLibrary.Delay` 25.0)
  (`|SpawnActorFromClass` "/Game/Blueprints/Abilities/AB_Ability_SacrificeAdds.AB_Ability_SacrificeAdds_C" (`self.GetTransform`) "Undefined" "MultiplyWithRoot" null self null)
  (`/Engine/EditorBlueprintResources/StandardMacros.IncrementInt` (`self.SacrificeCount`)
    (:`  `
      (if (or (`|EnumEquality` (`self.CurrentPhase`) "NewEnumerator2") (== (`self.SacrificeCount`) 2))
        (bind _returnvalue (`|SpawnActorFromClass` "/Game/Blueprints/Abilities/BP_ApocalypsePillar.BP_ApocalypsePillar_C" (`KismetMathLibrary.Conv_VectorToTransform` (- (+ (`self.K2_GetActorLocation`) (* (`self.GetActorForwardVector`) 1800.0)) (0.0 0.0 95.0))) "Undefined" "MultiplyWithRoot" null null))
        (set `self.ActivePillar` _returnvalue)
        (`KismetSystemLibrary.K2_SetTimerDelegate` (`|CreateDelegate` :!event `TriggerApocalypseBlast`) 20.0)))))

(event `self.Apply Damage`
  (params (Damage :type "Float (double-precision)") (`Damage Causer` :type "Actor Object Reference") (`Damage Location` :type "Vector Structure") (`Damage Impulse` :type "Vector Structure"))
  ; Health?
  (`/Game/Blueprints/BPC_Health.Apply Damage` (`self.BPC_Health`) Damage `Damage Causer` `Damage Location` `Damage Impulse`))

(event `TriggerSpinBeam`
  (bind _warning_cube (`self.Warning Cube`))
  ; Beam Spawn
  (`SceneComponent.SetVisibility` _warning_cube true true)
  (set `self.IsBusy` true)
  (`KismetSystemLibrary.Delay` (`.TelegraphDuration_33_AA3FA069480C5F91EFDC40BBA3FA789C` (break `/Game/Blueprints/F_AbiltyStruct` (`BlueprintMapLibrary.Map_Find` (`self.Abilities`) "NewEnumerator0"))))
  (`SceneComponent.SetVisibility` _warning_cube false true)
  (bind _returnvalue (`|SpawnActorFromClass` "/Game/Blueprints/Abilities/BP_Ability_LaserBeam.BP_Ability_LaserBeam_C" (`self.GetTransform`) "AlwaysSpawn" "MultiplyWithRoot" null self null))
  (set `self.ActiveBeam` _returnvalue)
  (`PrimitiveComponent.IgnoreActorWhenMoving` (`self.CapsuleComponent`) _returnvalue true)
  (`self.K2_AttachToComponent` (`self.ActiveBeam`) (`self.CapsuleComponent`) "None" "SnapToTarget" "SnapToTarget" "KeepWorld" true)
  (set `self.IsSpinning` true)
  (set `self.bUseControllerRotationYaw` false)
  (set `CharacterMovementComponent.bOrientRotationToMovement` false (`self.CharacterMovement`))
  (bind _returnvalue_2 (`KismetSystemLibrary.K2_SetTimerDelegate` (delegate `CheckDirectionChange`) 1.0 true))
  (`KismetSystemLibrary.K2_SetTimerDelegate` (`|CreateDelegate` :!event `EndLaserBeam`) (`.UseDuration_36_2D439E344E3C9A75B8300EA8431A69AB` (break `/Game/Blueprints/F_AbiltyStruct` (`BlueprintMapLibrary.Map_Find` (`self.Abilities`) "NewEnumerator0")))))

(event `EndLaserBeam`
  ; Beam Spawn
  (set `self.IsSpinning` false)
  (set `self.bUseControllerRotationYaw` true)
  (set `CharacterMovementComponent.bOrientRotationToMovement` true (`self.CharacterMovement`))
  (`self.K2_DestroyActor` (`self.ActiveBeam`))
  (`KismetSystemLibrary.K2_ClearAndInvalidateTimerHandle` (stale `TriggerSpinBeam` _returnvalue_2))
  (set `self.IsBusy` false)
  (add `self.OnDestroyed` (`|CreateDelegate` :!event `CustomEvent`)))

(event `CheckDirectionChange`
  ; Beam Spawn
  (if (< (`KismetMathLibrary.RandomFloatInRange` 0.0 1.0) 0.25)
    (set `self.SpinSpeed` (* (`self.SpinSpeed`) -1.0))))

(event `self.ReceiveTick`
  (params (DeltaSeconds :type "Float (single-precision)"))
  ; Beam Spawn
  ;; Tick Rotation
  (if (`self.IsSpinning`)
    (`self.K2_AddActorLocalRotation` (`KismetMathLibrary.MakeRotator` 0.0 0.0 (* DeltaSeconds (`self.SpinSpeed`))))
    (elif (not (`self.IsBusy`))
      (`self.K2_SetActorRotation` (`KismetMathLibrary.RInterpTo` (`self.K2_GetActorRotation`) (`KismetMathLibrary.MakeRotator` 0.0 0.0 (.yaw (`KismetMathLibrary.FindLookAtRotation` (`self.K2_GetActorLocation`) (`self.K2_GetActorLocation` (`GameplayStatics.GetPlayerCharacter` 0))))) DeltaSeconds 4.0)))))

(fn `UserConstructionScript`)