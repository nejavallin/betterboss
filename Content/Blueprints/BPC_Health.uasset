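; Health component that tracks its owner's health and broadcasts changes and death through event dispatchers.
; Health is set to MaxHealth one tick after BeginPlay, and damage and healing events forward to matching functions that fire OnHealthUpdated.
; Healing clamps the stored value, while damage clamps only the broadcast value.
; The death check subtracts damage a second time before firing OnDeath, which HandleDeath also triggers directly.
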(event `self.ReceiveBeginPlay`
  (`KismetSystemLibrary.DelayUntilNextTick`)
  (set `self.Health` (`self.MaxHealth`)))

(event `/Game/Blueprints/Interfaces/BPI_Damageable.Apply Healing`
  (params (Healing :type "Float (double-precision)") (Healer :type "Actor Object Reference"))
  (`self.ApplyHeal` Healing))

(event `/Game/Blueprints/Interfaces/BPI_Damageable.Apply Damage`
  (params (Damage :type "Float (double-precision)") (`Damage Causer` :type "Actor Object Reference") (`Damage Location` :type "Vector Structure") (`Damage Impulse` :type "Vector Structure"))
  (`self.ApplyDamage` Damage))

(event `/Game/Blueprints/Interfaces/BPI_Damageable.Handle Death`
  (`self.OnDeath`))

(fn `ApplyDamage`
  (params (Value :type "Float (double-precision)"))
  (bind _returnvalue (- (`self.Health`) Value))
  (bind _output_get (set `self.Health` _returnvalue))
  (`self.OnHealthUpdated` (`KismetMathLibrary.FClamp` _output_get 0.0 (`self.MaxHealth`)))
  (`KismetSystemLibrary.PrintString` "Hello")
  (if (<= _returnvalue 0.0)
    (`self.OnDeath`))
  (return))

(fn `ApplyHeal`
  (params (Value :type "Float (double-precision)"))
  (bind _output_get (set `self.Health` (`KismetMathLibrary.FClamp` (+ (`self.Health`) Value) 0.0 (`self.MaxHealth`))))
  (`self.OnHealthUpdated` _output_get)
  (return))