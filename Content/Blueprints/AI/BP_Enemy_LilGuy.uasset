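; BP_Enemy_LilGuy is an enemy whose attack fires a basic ranged projectile at its target.
; Attack turns the enemy to face a valid target, then spawns BP_BasicRanged just ahead of it, offset by its bounds, and passes a fixed value through SetVars.
; It calls CompleteAttack whether or not the target is valid.
; The event graph and construction script add no logic of their own.
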(fn `Attack`
  (params (Target :type "Actor Object Reference"))
  (bind (_origin _boxextent) (`self.GetActorBounds` false))
  (bind _returnvalue (`KismetMathLibrary.FindLookAtRotation` (`self.K2_GetActorLocation`) (`self.K2_GetActorLocation` Target)))
  (`/Engine/EditorBlueprintResources/StandardMacros.IsValid` Target
    (:`Is Valid`
      (`self.K2_SetActorRotation` _returnvalue)
      (bind _returnvalue_2 (`|SpawnActorFromClass` "/Game/Blueprints/Abilities/BP_BasicRanged.BP_BasicRanged_C" (`KismetMathLibrary.MakeTransform` (+ (`self.K2_GetActorLocation`) (* (`self.GetActorForwardVector`) (`KismetMathLibrary.MakeVector` (.x _boxextent) (.x _boxextent) 1.0))) _returnvalue) "AdjustIfPossibleButAlwaysSpawn" "MultiplyWithRoot" null self))
      (`/Game/Blueprints/Abilities/BP_BasicRanged.SetVars` _returnvalue_2 10.0)
      (`self.CompleteAttack`)
      (return))
    (:`Is Not Valid`
      (`self.CompleteAttack`)
      (return))))

(fn `UserConstructionScript`
  (`parent.UserConstructionScript`))