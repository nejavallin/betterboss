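; BP_TestEnemy is a test enemy with a lunge-style attack that damages what lies ahead.
; Attack runs an oriented box overlap along its forward vector, applies damage through BPC_Health components and draws debug output.
; AttackComplete waits, teleports the enemy up to attack distance toward the target's direction, then signals completion after recovery.
; Construction derives AttackRange from attack distance and a trigger multiplier.
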(event `AttackComplete`
  (params (NewPos :type "Vector Structure"))
  (`KismetSystemLibrary.Delay` (`self.AttackDuration`))
  (`self.K2_SetActorLocation` NewPos false true)
  (`KismetSystemLibrary.Delay` (`self.RecoveryDuration`))
  (`self.OnAttackComplete`))

(event `self.Sphere.OnComponentBeginOverlap`
  (params (OverlappedComponent :type "PrimitiveComponent Object Reference") (OtherActor :type "Actor Object Reference") (OtherComp :type "PrimitiveComponent Object Reference") (OtherBodyIndex :type Integer) (bFromSweep :type Boolean) (SweepResult :type "HitResult Structure (by ref)")))

(fn `Attack`
  (params (Target :type "Actor Object Reference"))
  (locals (NewLocalVar :type "Array of Actor Object Reference") (NewLocalVar_0 :type "Array of EObjectTypeQuery Enum") (LocalTarget :type "Actor Object Reference") (EndPos :type "Vector Structure") (Hits :type "Array of Actor Object Reference"))
  (bind _returnvalue (`self.K2_GetActorLocation`))
  (bind _returnvalue_2 (`self.K2_GetActorRotation`))
  (bind (_attackbounds_x _attackbounds_y) (`KismetMathLibrary.BreakVector2D` (`self.AttackBounds`)))
  (bind _attackdistance (`self.AttackDistance`))
  (bind _attackdistance_2 (`self.AttackDistance`))
  (bind _returnvalue_3 (`KismetMathLibrary.MakeVector` (* _attackdistance_2 0.5) _attackbounds_x _attackbounds_y))
  (bind _returnvalue_4 (+ (`self.K2_GetActorLocation`) (* (* (`self.GetActorForwardVector`) _attackdistance_2) 0.5)))
  (set `local.LocalTarget` Target)
  (set `local.EndPos` (+ (* (`KismetMathLibrary.Normal` (- (`self.K2_GetActorLocation` Target) _returnvalue)) (`KismetMathLibrary.MakeVector` _attackdistance _attackdistance 1.0)) _returnvalue))
  (bind _outactors (`KismetSystemLibrary.BoxOverlapActorsWithOrientation` _returnvalue_4 _returnvalue_3 _returnvalue_2 (`|MakeArray` "ObjectTypeQuery2" "ObjectTypeQuery3" :!type "EObjectTypeQuery Enum")))
  (set `local.Hits` _outactors)
  (`KismetSystemLibrary.DrawDebugBox` _returnvalue_4 _returnvalue_3 (struct :`R` 0.089799 :`G` 1.0 :`B` 0.272426 :`A` 1.0) _returnvalue_2 2.0 5.0)
  (for _array_element (`local.Hits`)
    (bind _returnvalue_5 (`self.GetComponentByClass` _array_element "/Game/Blueprints/BPC_Health.BPC_Health_C"))
    (`/Engine/EditorBlueprintResources/StandardMacros.IsValid` _returnvalue_5
      (:`Is Valid`
        (`/Game/Blueprints/BPC_Health.ApplyDamage` _returnvalue_5 (`self.Damage`)))))
  (`KismetSystemLibrary.PrintString` "--ATTACK--" true true (struct :`R` 0.291938 :`G` 1.0 :`B` 0.149059 :`A` 1.0))
  (`self.AttackComplete` (`local.EndPos`))
  (return))

(fn `UserConstructionScript`
  (set `self.AttackRange` (* (`self.AttackDistance`) (`self.AttackTriggerRange%`))))