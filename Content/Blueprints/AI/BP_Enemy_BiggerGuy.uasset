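; Larger enemy Blueprint with a lightning dash attack and a camera-facing health bar driven by its health component.
; Attack damages every actor with BPC_Health in an oriented box ahead (debug-drawn), then sends a Niagara trail forward, teleports after AttackDuration and calls OnStageComplete.
; Unless ActiveOnSpawn is set, BeginPlay stores and unpossesses its controller, which RepossesSelf can later restore.
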(event `self.ReceiveTick`
  (params (DeltaSeconds :type "Float (single-precision)"))
  (bind _biggerenemyhealthbar (`self.BiggerEnemyHealthBar`))
  ; Health bar always visable
  (`SceneComponent.K2_SetWorldRotation` _biggerenemyhealthbar (`KismetMathLibrary.FindLookAtRotation` (`SceneComponent.K2_GetComponentLocation` _biggerenemyhealthbar) (`PlayerCameraManager.GetCameraLocation` (`GameplayStatics.GetPlayerCameraManager` 0))) false false))

(event `OnBiggerEnemyHealthUpdated`
  (params (NewHealth :type "Float (double-precision) (by ref)"))
  (`/Game/UI/WBP_BiggerEnemyHealthBar.UpdateBiggerEnemyHealth` (`self.Bigger Enemy HUD`) NewHealth (`/Game/Blueprints/Components/BPC_Health.MaxHealth` (`self.BPC_Health`))))

(event `self.ReceiveBeginPlay`
  (bind _returnvalue (`self.GetController`))
  (`|ExecutionSequence`
    (:`then_0`
      (`parent.ReceiveBeginPlay`)
      (if (not (`self.ActiveOnSpawn`))
        (set `self.StartomgController` _returnvalue)
        (`Controller.UnPossess` _returnvalue)))
    (:`then_1`
      (bind _aswbp_bigger_enemy_health_bar (cast `/Game/UI/WBP_BiggerEnemyHealthBar` (`WidgetComponent.GetUserWidgetObject` (`self.BiggerEnemyHealthBar`))))
      (set `self.Bigger Enemy HUD` _aswbp_bigger_enemy_health_bar)
      (add `/Game/Blueprints/Components/BPC_Health.OnHealthUpdated` (`self.BPC_Health`) (delegate `OnBiggerEnemyHealthUpdated`))
      (`/Game/UI/WBP_BiggerEnemyHealthBar.UpdateBiggerEnemyHealth` (`self.Bigger Enemy HUD`) (`/Game/Blueprints/Components/BPC_Health.Health` (`self.BPC_Health`)) (`/Game/Blueprints/Components/BPC_Health.MaxHealth` (`self.BPC_Health`))))))

(event `AttackComplete`
  (params (NewPos :type "Vector Structure"))
  (bind _returnvalue (`self.K2_GetActorLocation`))
  (bind _returnvalue_2 (`KismetMathLibrary.FindLookAtRotation` _returnvalue NewPos))
  (bind _returnvalue_3 (`NiagaraFunctionLibrary.SpawnSystemAtLocation` "/Game/__LightningThunderVFX/NS/NS_Trail_LightningSlash.NS_Trail_LightningSlash" _returnvalue _returnvalue_2))
  (`GameplayStatics.PlaySoundAtLocation` "/Game/SFX/dashing_add.dashing_add" (`self.K2_GetActorLocation`) (struct) 1.0 1.0 0.0 "/Game/SFX/Attenuation.Attenuation" null null null)
  (`KismetSystemLibrary.MoveComponentTo` _returnvalue_3 NewPos _returnvalue_2 false false 0.1)
  (`KismetSystemLibrary.Delay` (`self.AttackDuration`))
  (`self.K2_SetActorLocation` NewPos false true)
  (`ActorComponent.K2_DestroyComponent` _returnvalue_3)
  (`self.OnStageComplete`))

(fn `Attack`
  (params (Target :type "Actor Object Reference"))
  (locals (Local_Target :type "Actor Object Reference") (EndPos :type "Vector Structure") (Hits :type "Array of Actor Object Reference"))
  (bind _returnvalue (`self.GetActorForwardVector`))
  (bind _returnvalue_2 (`self.K2_GetActorRotation`))
  (bind _returnvalue_3 (`self.K2_GetActorLocation`))
  (bind _attackdistance (`self.AttackDistance`))
  (bind _attackdistance_2 (`self.AttackDistance`))
  (bind (_attackbounds_x _attackbounds_y) (`KismetMathLibrary.BreakVector2D` (`self.AttackBounds`)))
  (bind _returnvalue_4 (`KismetMathLibrary.MakeVector` (* _attackdistance 0.5) _attackbounds_x _attackbounds_y))
  (bind _returnvalue_5 (+ (* (* _returnvalue _attackdistance) 0.5) _returnvalue_3))
  (`GameplayStatics.PlaySoundAtLocation` "/Game/__LightningThunderVFX/_GenericSource/SFX/Sfx_Hit_Thunder_short.Sfx_Hit_Thunder_short" (`self.K2_GetActorLocation`) (struct) 1.0 1.0 0.0 "/Game/SFX/Attenuation.Attenuation" null null null)
  (set `local.Local_Target` Target)
  (set `local.EndPos` (+ _returnvalue_3 (* _returnvalue (`KismetMathLibrary.MakeVector` _attackdistance_2 _attackdistance_2 1.0))))
  (bind _outactors (`KismetSystemLibrary.BoxOverlapActorsWithOrientation` _returnvalue_5 _returnvalue_4 _returnvalue_2 (`|MakeArray` "ObjectTypeQuery2" "ObjectTypeQuery3" "ObjectTypeQuery1" :!type "EObjectTypeQuery Enum")))
  (bind _output_get (set `local.Hits` _outactors))
  (`KismetSystemLibrary.DrawDebugBox` _returnvalue_5 _returnvalue_4 (struct :`R` 0.089799 :`G` 1.0 :`B` 0.272426 :`A` 1.0) _returnvalue_2 2.0 5.0)
  (for _array_element _output_get
    (bind _returnvalue_6 (`self.GetComponentByClass` _array_element "/Game/Blueprints/Components/BPC_Health.BPC_Health_C"))
    (`/Engine/EditorBlueprintResources/StandardMacros.IsValid` _returnvalue_6
      (:`Is Valid`
        (`/Game/Blueprints/Components/BPC_Health.ApplyDamage` _returnvalue_6 (`self.Damage`)))))
  (`self.AttackComplete` (`local.EndPos`))
  (return))

(fn `RepossesSelf`
  (`Controller.Possess` (`self.StartomgController`) self))

(fn `UnPosses`
  (`Controller.UnPossess` (`self.StartomgController`)))

(fn `UserConstructionScript`
  (`parent.UserConstructionScript`))