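; Base enemy actor that passes its health to a health component and, on death, plays an optional montage before destroying itself.
; AttackSequanceStage routes windup, attack and recovery stages, each signaling completion through CallOnStageComplete.
; Windup and recovery have optional timed defaults, with the telegraph ball turning red during windup.
; Attack only prints debug text before a timed completion, and attack range is a percentage of attack distance.
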(event `self.ReceiveBeginPlay`
  (set `self.AttackRange` (* (`self.AttackDistance`) (* (`self.AttackTriggerRange%`) 0.01)))
  (set `/Game/Blueprints/BPC_Health.Health` (`self.Health`) (`self.BPC_Health`)))

(event `self.BPC_Health.OnDeath`
  (bind _deathanim (`self.DeathAnim`)
    (:`then`
      (bind _returnvalue (`self.PlayAnimMontage` _deathanim))
      (`KismetSystemLibrary.Delay` _returnvalue))
    (:`else`
      _))
  (`self.K2_DestroyActor`))

(event `CompleteAttack`
  (`KismetSystemLibrary.Delay` (`self.AttackDuration`))
  (`self.OnStageComplete`))

(event `Telegrapgh`
  (params (UseDefault :type Boolean))
  (if UseDefault
    (`PrimitiveComponent.SetMaterial` (`self.TelegraphBall`) 0 "/Game/Materials/Red.Red")
    (`KismetSystemLibrary.Delay` (`self.TelegrapthDuration`))
    (`PrimitiveComponent.SetMaterial` (`self.TelegraphBall`) 0 "/Game/Variant_Combat/Materials/M_Lava.M_Lava"))
  (`self.OnStageComplete`))

(event `RecoverEvent`
  (if (`self.UseDefaultTelegraphRecover`)
    (`KismetSystemLibrary.Delay` (`self.RecoveryDuration`)))
  (`self.OnStageComplete`))

(fn `Attack`
  (params (Target :type "Actor Object Reference"))
  (locals (NewLocalVar :type "Array of Actor Object Reference") (NewLocalVar_0 :type "Array of EObjectTypeQuery Enum") (LocalTarget :type "Actor Object Reference") (EndPos :type "Vector Structure") (Hits :type "Array of Actor Object Reference"))
  (`KismetSystemLibrary.PrintText` (`|FormatText` "--Attack-- \n{target} was attacked in range {range}" Target (`self.GetDistanceTo` Target)) true true (struct :`R` 1.0 :`G` 0.143505 :`B` 0.01928 :`A` 1.0) 3.0)
  (`self.CompleteAttack`)
  (return))

(fn `AttackSequanceStage`
  (params (Stage :type "/Game/Blueprints/AI/E_AttackSequence Enum" :default "NewEnumerator0") (AttackTarget :type "Actor Object Reference"))
  (bind _output_get (set `self.Attack Target` AttackTarget))
  (switch `/Game/Blueprints/AI/E_AttackSequence` Stage
    (:`NewEnumerator0`
      (`self.Telegrapgh` (`self.UseDefaultTelegraphRecover`)))
    (:`NewEnumerator1`
      (`self.Attack` _output_get))
    (:`NewEnumerator2`
      (`self.RecoverEvent`))))

(fn `UserConstructionScript`
  (set `self.AttackRange` (* (`self.AttackDistance`) (* (`self.AttackTriggerRange%`) 0.01))))