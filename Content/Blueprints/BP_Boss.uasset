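; Boss enemy that runs three health-driven phases, shows a health bar widget and turns to face the player when not casting or spinning.
; Health updates advance the phase and restart the looping ability timer.
; ChooseAbility picks a cone attack (only a debug print) or, in later phases, a cooldown-gated laser beam spin with random direction flips.
; Summoning spawns minions around the boss, with a delayed sacrifice ability outside the first phase.
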(event `ResetBeamCooldown`
  (set `self.bCanCastBeam` true)
  (set `self.bCanCastBeam` false :!label _label)
  (`KismetSystemLibrary.K2_SetTimerDelegate` (`|CreateDelegate` :!event `ResetBeamCooldown`) 30.0)
  (`self.TriggerSpinBeam`))

(event `ChooseAbility`
  (if (not (`self.IsCasting`))
    (`/Engine/EditorBlueprintResources/StandardMacros.IsValid` (`self.PlayerRef`)
      (:`Is Valid`
        _)
      (:`Is Not Valid`
        (bind _asbp_player_char (cast `/Game/Blueprints/Player/BP_PlayerChar` (`GameplayStatics.GetPlayerCharacter` 0)))
        (set `self.PlayerRef` _asbp_player_char)))
    (switch `/Game/Blueprints/E_BossPhase` (`self.CurrentPhase`)
      (:`NewEnumerator0`
        (`self.TriggerConeAttack`))
      (:`NewEnumerator1`
        (if (`self.bCanCastBeam`) :!label _label_2
          (goto _label)
          (else
            (`self.TriggerConeAttack`))))
      (:`NewEnumerator2`
        (goto _label_2)))))

(event `TriggerConeAttack`
  (`KismetSystemLibrary.PrintString` "Boss casts cone attack!"))

(event `self.ReceiveBeginPlay`
  (`|ExecutionSequence`
    (:`then_0`
      ; HealthBar
      (bind _returnvalue (`|CreateWidget` "/Game/UI/WBP_BossHealthBar.WBP_BossHealthBar_C" (`GameplayStatics.GetPlayerController` 0)))
      (bind _output_get (set `self.BossHealthBar` _returnvalue))
      (`UserWidget.AddToViewport` _output_get 0)
      (add `/Game/Blueprints/BPC_Health.OnHealthUpdated` (`self.BPC_Health`) (delegate `UpdateHealthBar`))
      (add `/Game/Blueprints/BPC_Health.OnDeath` (`self.BPC_Health`) (delegate `OnBossDeath`))
      (bind _asbp_player_char (cast `/Game/Blueprints/Player/BP_PlayerChar` (`GameplayStatics.GetPlayerCharacter` 0)))
      (set `self.PlayerRef` _asbp_player_char)
      (bind _returnvalue_2 (`KismetSystemLibrary.K2_SetTimerDelegate` (`|CreateDelegate` :!event `ChooseAbility`) (`self.AbilityCooldown`) true))
      (set `self.AbilityCooldownTimer` _returnvalue_2)
      (`KismetSystemLibrary.K2_SetTimerDelegate` (`|CreateDelegate` :!event `TriggerSummonAdds`) 2.0))))

(event `UpdateHealthBar`
  (params (NewHealth :type "Float (double-precision) (by ref)"))
  (bind _bpc_health (`self.BPC_Health`))
  (bind _returnvalue (/ (`/Game/Blueprints/BPC_Health.Health` _bpc_health) (`/Game/Blueprints/BPC_Health.MaxHealth` _bpc_health)))
  ; HealthBar
  (`/Game/UI/WBP_BossHealthBar.Boss Set Life Percentage` (`self.BossHealthBar`) _returnvalue)
  (if (and (<= _returnvalue 0.65) (`|EnumEquality` (`self.CurrentPhase`) "NewEnumerator0"))
    (set `self.CurrentPhase` "NewEnumerator1")
    (`KismetSystemLibrary.K2_ClearAndInvalidateTimerHandle` (`self.AbilityCooldownTimer`))
    (bind _returnvalue_2 (`KismetSystemLibrary.K2_SetTimerDelegate` (`|CreateDelegate` :!event `ChooseAbility`) 5.0 true))
    (set `self.AbilityCooldownTimer` _returnvalue_2)
    (`KismetSystemLibrary.K2_SetTimerDelegate` (`|CreateDelegate` :!event `TriggerSummonAdds`) 3.0)
    (elif (and (<= _returnvalue 0.3) (`|EnumEquality` (`self.CurrentPhase`) "NewEnumerator1"))
      (set `self.CurrentPhase` "NewEnumerator2")
      (`KismetSystemLibrary.K2_ClearAndInvalidateTimerHandle` (`self.AbilityCooldownTimer`))
      (bind _returnvalue_3 (`KismetSystemLibrary.K2_SetTimerDelegate` (`|CreateDelegate` :!event `ChooseAbility`) 2.0 true))
      (set `self.AbilityCooldownTimer` _returnvalue_3)
      (`KismetSystemLibrary.K2_SetTimerDelegate` (`|CreateDelegate` :!event `TriggerSummonAdds`) 10.0))))

(event `OnBossDeath`
  ; HealthBar
  (`Widget.RemoveFromParent` (`self.BossHealthBar`)))

(event `TriggerSummonAdds`
  (bind (_returnvalue_x _returnvalue_y) (`KismetMathLibrary.BreakVector` (`KismetMathLibrary.RandomUnitVector`)))
  ; spawn adds
  (set `self.IsCasting` true)
  (`NiagaraFunctionLibrary.SpawnSystemAtLocation` "/Game/VFX/Mixed_Magic_VFX_Pack/VFX/NS_Dark_Owner_Cast_Spell.NS_Dark_Owner_Cast_Spell" (`self.K2_GetActorLocation`))
  (`KismetSystemLibrary.Delay` 2.0)
  (set `self.IsCasting` false)
  (for _ (range 6)
    (`|SpawnActorFromClass` "/Game/Blueprints/AI/BP_Enemy_LilGuy.BP_Enemy_LilGuy_C" (`KismetMathLibrary.MakeTransform` (+ (* (`KismetMathLibrary.MakeVector` _returnvalue_x _returnvalue_y) 5000.0) (`self.K2_GetActorLocation`))) "Undefined" "MultiplyWithRoot" null null)
    (`self.SpawnDefaultController`))
  (if (!= (`self.CurrentPhase`) 1)
    (`KismetSystemLibrary.Delay` 10.0)
    (`|SpawnActorFromClass` "/Game/Blueprints/Abilities/AB_Ability_SacrificeAdds.AB_Ability_SacrificeAdds_C" (`self.GetTransform`) "Undefined" "MultiplyWithRoot" null self null)))

(event `/Game/Blueprints/Interfaces/BPI_Damageable.Apply Damage`
  (params (Damage :type "Float (double-precision)") (`Damage Causer` :type "Actor Object Reference") (`Damage Location` :type "Vector Structure") (`Damage Impulse` :type "Vector Structure"))
  ; Health?
  (`/Game/Blueprints/BPC_Health.Apply Damage` (`self.BPC_Health`) Damage `Damage Causer` `Damage Location` `Damage Impulse`))

(event `TriggerSpinBeam`
  (bind _warning_cube (`self.Warning Cube`))
  ; Beam Spawn
  (`SceneComponent.SetVisibility` _warning_cube true false)
  (set `self.IsCasting` true)
  (`KismetSystemLibrary.Delay` 2.0)
  (set `self.IsCasting` false)
  (`SceneComponent.SetVisibility` _warning_cube false false)
  (bind _returnvalue (`|SpawnActorFromClass` "/Game/Blueprints/Abilities/BP_Ability_LaserBeam.BP_Ability_LaserBeam_C" (`self.GetTransform`) "AlwaysSpawn" "MultiplyWithRoot" null null))
  (set `self.ActiveBeam` _returnvalue)
  (`PrimitiveComponent.IgnoreActorWhenMoving` (`self.CapsuleComponent`) _returnvalue true)
  (`self.K2_AttachToComponent` (`self.ActiveBeam`) (`self.CapsuleComponent`) "None" "SnapToTarget" "SnapToTarget" "KeepWorld" true)
  (set `self.IsSpinning` true)
  (set `self.bUseControllerRotationYaw` false)
  (set `CharacterMovementComponent.bOrientRotationToMovement` false (`self.CharacterMovement`))
  (bind _returnvalue_2 (`KismetSystemLibrary.K2_SetTimerDelegate` (delegate `CheckDirectionChange`) 1.0 true))
  (`KismetSystemLibrary.Delay` 10.0)
  (set `self.IsSpinning` false)
  (set `self.bUseControllerRotationYaw` true)
  (set `CharacterMovementComponent.bOrientRotationToMovement` true (`self.CharacterMovement`))
  (`self.K2_DestroyActor` (`self.ActiveBeam`))
  (`KismetSystemLibrary.K2_ClearAndInvalidateTimerHandle` _returnvalue_2))

(event `CheckDirectionChange`
  ; Beam Spawn
  (if (< (`KismetMathLibrary.RandomFloatInRange` 0.0 1.0) 0.25)
    (set `self.SpinSpeed` (* (`self.SpinSpeed`) -1.0))))

(event `self.ReceiveTick`
  (params (DeltaSeconds :type "Float (single-precision)"))
  ; Beam Spawn
  ;; Tick Rotation
  (if (`self.IsSpinning`)
    (`self.K2_AddActorLocalRotation` (`KismetMathLibrary.MakeRotator` 0.0 0.0 (* DeltaSeconds (`self.SpinSpeed`))))
    (elif (not (`self.IsCasting`))
      (`self.K2_SetActorRotation` (`KismetMathLibrary.RInterpTo` (`self.K2_GetActorRotation`) (`KismetMathLibrary.MakeRotator` 0.0 0.0 (.yaw (`KismetMathLibrary.FindLookAtRotation` (`self.K2_GetActorLocation`) (`self.K2_GetActorLocation` (`GameplayStatics.GetPlayerCharacter` 0))))) DeltaSeconds 4.0)))))

(fn `UserConstructionScript`)