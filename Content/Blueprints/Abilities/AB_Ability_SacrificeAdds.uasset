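; Boss ability actor that sacrifices LilGuy enemies one at a time to heal the boss.
; BeginPlay shows taunt text, marks the boss busy, attaches electric VFX and, after a delay, starts a looping timer.
; Each SacrificeOneAdd destroys one add with a hit effect and applies healing.
; When none remain, it clears the timer, frees the non-spinning boss and destroys itself; the aura reference it cleans up is never assigned.
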(event `SacrificeOneAdd`
  (bind _outactors (`GameplayStatics.GetAllActorsOfClass` "/Game/Blueprints/AI/BP_Enemy_LilGuy.BP_Enemy_LilGuy_C"))
  (if (> (`KismetArrayLibrary.Array_Length` _outactors) 0)
    (bind _output (`|GetArrayItem` _outactors))
    (`NiagaraFunctionLibrary.SpawnSystemAtLocation` "/Game/__LightningThunderVFX/NS/NS_Hit_Electric_01AA.NS_Hit_Electric_01AA" (`self.K2_GetActorLocation` _output))
    (`self.K2_DestroyActor` _output)
    (`/Game/Blueprints/Components/BPC_Health.ApplyHeal` (`/Game/Blueprints/BP_Boss.BPC_Health` (`self.BossRef`)) 35.0)
    (else
      (`KismetSystemLibrary.K2_ClearAndInvalidateTimerHandle` (`self.SacrificeTimerHandle`))
      (bind _outactors_2 (`GameplayStatics.GetAllActorsOfClass` "/Game/Blueprints/AI/BP_Enemy_LilGuy.BP_Enemy_LilGuy_C"))
      (for _array_element _outactors_2
        (`self.K2_DestroyActor` _array_element))
      (`ActorComponent.K2_DestroyComponent` (`self.AuraVFXRef`))
      (if (not (`/Game/Blueprints/BP_Boss.IsSpinning` (`self.BossRef`)))
        (set `/Game/Blueprints/BP_Boss.IsBusy` false (`self.BossRef`)))
      (`self.K2_DestroyActor`))))

(event `self.ReceiveBeginPlay`
  ; Text
  (bind _asbp_player_char (cast `/Game/Blueprints/Player/BP_PlayerChar` (`GameplayStatics.GetPlayerCharacter` 0)))
  (`/Game/Blueprints/Player/BP_PlayerChar.ShowOpeningCutsceneText` _asbp_player_char "My Followers give your life to me" 5.0)
  (set `/Game/Blueprints/BP_Boss.IsBusy` true (`self.BossRef`))
  (bind _returnvalue (`NiagaraFunctionLibrary.SpawnSystemAttached` "/Game/__LightningThunderVFX/NS/NS_Hit_Electric_01AA.NS_Hit_Electric_01AA" (`Character.Mesh` (`self.BossRef`)) "pelvis" (0.0 0.0 0.0) (struct :`Pitch` 90.0 :`Roll` 90.0) "SnapToTarget" true))
  (`KismetSystemLibrary.Delay` 3.0)
  (bind _returnvalue_2 (`KismetSystemLibrary.K2_SetTimerDelegate` (`|CreateDelegate` :!event `SacrificeOneAdd`) 1.0 true))
  (set `self.SacrificeTimerHandle` _returnvalue_2))

(fn `UserConstructionScript`)