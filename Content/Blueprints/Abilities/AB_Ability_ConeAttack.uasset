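; AB_Ability_ConeAttack is a short-lived boss ability actor that delivers a telegraphed forward attack.
; On BeginPlay it marks BossRef busy and shows a hand-attached Niagara telegraph during a wind-up delay.
; It then spawns forward VFX and runs a single-hit box trace for Pawns, a swept box despite the cone name, applying damage through BPC_Health.
; After a recovery delay it clears the busy flag and destroys itself.
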(event `self.ReceiveBeginPlay`
  (bind _returnvalue (`self.K2_GetActorRotation` (`self.BossRef`)))
  (set `/Game/Blueprints/BP_Boss.IsBusy` true (`self.BossRef`))
  (bind _returnvalue_2 (`NiagaraFunctionLibrary.SpawnSystemAttached` "/Game/__LightningThunderVFX/NS/NS_BolasAxe.NS_BolasAxe" (`Character.Mesh` (`self.BossRef`)) "hand_r" (0.0 0.0 0.0) (struct) "SnapToTarget"))
  (set `self.TelegraphVFXRef` _returnvalue_2)
  (`KismetSystemLibrary.Delay` 1.5)
  (`ActorComponent.K2_DestroyComponent` (`self.TelegraphVFXRef`))
  (`NiagaraFunctionLibrary.SpawnSystemAtLocation` "/Game/__LightningThunderVFX/NS/NS_Line_RamuhWalk.NS_Line_RamuhWalk" (+ (`self.K2_GetActorLocation` (`self.BossRef`)) (* (`self.GetActorForwardVector` (`self.BossRef`)) 200.0)) _returnvalue)
  (bind _outhit (`KismetSystemLibrary.BoxTraceSingleForObjects` (`self.K2_GetActorLocation` (`self.BossRef`)) (+ (* (`SceneComponent.GetForwardVector` (`Actor.RootComponent` (`self.BossRef`))) 800.0) (`self.K2_GetActorLocation` (`self.BossRef`))) (150.0 150.0 150.0) _returnvalue (`|MakeArray` "ObjectTypeQuery3" :!type "EObjectTypeQuery Enum")))
  (`/Game/Blueprints/BPC_Health.Apply Damage` (`self.GetComponentByClass` (`.HitActor` (`GameplayStatics.BreakHitResult` _outhit)) "/Game/Blueprints/BPC_Health.BPC_Health_C") 5.0 null (0.0 0.0 0.0) (0.0 0.0 0.0))
  (`KismetSystemLibrary.Delay` 1.5)
  (set `/Game/Blueprints/BP_Boss.IsBusy` false (`self.BossRef`))
  (`self.K2_DestroyActor`))

(fn `UserConstructionScript`)