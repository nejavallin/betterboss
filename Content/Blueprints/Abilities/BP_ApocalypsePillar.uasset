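; BP_ApocalypsePillar is a telegraphed falling-pillar ability that knocks the player away and leaves a solid pillar behind.
; On BeginPlay it hides the mesh and shows a runic Niagara warning for a few seconds.
; It then sphere-traces for pawns and launches a hit BP_PlayerChar outward and upward before the drop begins, without applying damage.
; A timeline lerps the mesh down, then triggers impact VFX, camera shake and collision.
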(event `self.ReceiveBeginPlay`
  (bind _returnvalue (`self.K2_GetActorLocation`))
  (`PrimitiveComponent.SetCollisionEnabled` (`self.StaticMesh`) "NoCollision")
  (`SceneComponent.SetVisibility` (`self.StaticMesh`) false false)
  (bind _returnvalue_2 (`NiagaraFunctionLibrary.SpawnSystemAtLocation` "/Game/MagicCircles/FX/Runic/NS_Runic_02.NS_Runic_02" (- (`self.K2_GetActorLocation`) (0.0 0.0 250.0)) (struct) (5.0 5.0 5.0)))
  (set `self.TelegraphVFXRef` _returnvalue_2)
  (`KismetSystemLibrary.Delay` 4.0)
  (`ActorComponent.K2_DestroyComponent` (`self.TelegraphVFXRef`))
  (bind _outhit (`KismetSystemLibrary.SphereTraceSingleForObjects` _returnvalue _returnvalue 500.0 (`|MakeArray` "ObjectTypeQuery3" :!type "EObjectTypeQuery Enum")))
  (bind _asbp_player_char (cast `/Game/Blueprints/Player/BP_PlayerChar` (`.HitActor` (`GameplayStatics.BreakHitResult` _outhit)))
    (:`then`
      (`Character.LaunchCharacter` _asbp_player_char (+ (* (`KismetMathLibrary.Normal` (- (`self.K2_GetActorLocation` _asbp_player_char) (`self.K2_GetActorLocation`))) 3500.0) (0.0 0.0 800.0)) true true))
    (:`CastFailed`
      _))
  (`SceneComponent.SetVisibility` (`self.StaticMesh`) true false)
  (bind (_direction _alpha) (`Timeline|PillarDropTimeline` :!via `PlayFromStart`)
    (:`Update`
      (`SceneComponent.K2_SetWorldLocation` (`self.StaticMesh`) (`KismetMathLibrary.VLerp` (+ (`self.K2_GetActorLocation`) (0.0 0.0 3500.0)) (- (`self.K2_GetActorLocation`) (0.0 0.0 250.0)) _alpha) false false))
    (:`Finished`
      (`NiagaraFunctionLibrary.SpawnSystemAtLocation` "/Game/VFX/Mixed_Magic_VFX_Pack/VFX/NS_Big_Hammer_Impact.NS_Big_Hammer_Impact" _returnvalue)
      (`PlayerCameraManager.StartCameraShake` :`self` (`GameplayStatics.GetPlayerCameraManager` 0) :`ShakeClass` "/Game/Variant_Combat/Blueprints/BP_CameraShake_Hit_Player.BP_CameraShake_Hit_Player_C" :`Scale` 5.0)
      (`PrimitiveComponent.SetCollisionEnabled` (`self.StaticMesh`) "QueryAndPhysics"))))

(fn `UserConstructionScript`)