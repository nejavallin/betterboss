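; Boss ability actor for Apocalypse Blast, a charged attack that runs on BeginPlay and destroys itself when done.
; A timeline levitates the busy boss, then a charge effect plays through a delay before the blast.
; A sphere trace toward the player damages and launches them if hit; otherwise the referenced pillar is destroyed with an impact effect.
; The boss then returns to its start location, resumes walking and clears its busy flag.
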(event `self.ReceiveBeginPlay`
  (bind _bossref (`self.BossRef`))
  (bind _playerref (`/Game/Blueprints/BP_Boss.PlayerRef` (`self.BossRef`)))
  (set `/Game/Blueprints/BP_Boss.IsBusy` true (`self.BossRef`))
  (set `self.BossStartLocation` (`self.K2_GetActorLocation` (`self.BossRef`)))
  (`CharacterMovementComponent.SetMovementMode` (`Character.CharacterMovement` (`self.BossRef`)) "MOVE_None" 0)
  (bind (_direction _alpha) (`Timeline|LevitateTimeLine` :!via `PlayFromStart`)
    (:`Update`
      (`self.K2_SetActorLocation` (`self.BossRef`) (`KismetMathLibrary.VLerp` (`self.BossStartLocation`) (+ (`self.BossStartLocation`) (0.0 0.0 300.0)) _alpha) false false))
    (:`Finished`
      (bind _returnvalue (`NiagaraFunctionLibrary.SpawnSystemAtLocation` "/Game/__LightningThunderVFX/NS/NS_Hit_Constant_IonLaserAA.NS_Hit_Constant_IonLaserAA" (`self.K2_GetActorLocation` (`self.BossRef`)) (struct) (3.0 3.0 3.0)))
      (set `self.ChargeVFXRef` _returnvalue)
      (`KismetSystemLibrary.Delay` 5.0)
      (`ActorComponent.K2_DestroyComponent` (`self.ChargeVFXRef`))
      (`NiagaraFunctionLibrary.SpawnSystemAtLocation` "/Game/VFX/Mixed_Magic_VFX_Pack/VFX/NS_Potion.NS_Potion" (`self.K2_GetActorLocation` (`self.BossRef`)) (struct) (100.0 100.0 100.0))
      (bind _outhit (`KismetSystemLibrary.SphereTraceSingleForObjects` (+ (`self.K2_GetActorLocation` (`self.BossRef`)) (0.0 0.0 300.0)) (`self.K2_GetActorLocation` _playerref) 450.0 (`|MakeArray` "ObjectTypeQuery3" "ObjectTypeQuery2" "ObjectTypeQuery1" :!type "EObjectTypeQuery Enum")))
      (bind _asbp_player_char (cast `/Game/Blueprints/Player/BP_PlayerChar` (`.HitActor` (`GameplayStatics.BreakHitResult` _outhit)))
        (:`then`
          (`/Game/Blueprints/BPC_Health.ApplyDamage` (`self.GetComponentByClass` _asbp_player_char "/Game/Blueprints/BPC_Health.BPC_Health_C") 80.0)
          (`Character.LaunchCharacter` _asbp_player_char (+ (* (`KismetMathLibrary.Normal` (`KismetMathLibrary.MakeVector` (.x (- (`self.K2_GetActorLocation` _playerref) (`self.K2_GetActorLocation` (`self.BossRef`)))) (.y (- (`self.K2_GetActorLocation` _playerref) (`self.K2_GetActorLocation` (`self.BossRef`)))))) 7000.0) (0.0 0.0 1800.0)) true true))
        (:`CastFailed`
          (`NiagaraFunctionLibrary.SpawnSystemAtLocation` "/Game/VFX/Mixed_Magic_VFX_Pack/VFX/NS_Big_Hammer_Impact.NS_Big_Hammer_Impact" (`self.K2_GetActorLocation` (`self.PillarRef`)) (struct) (3.0 3.0 3.0))
          (`self.K2_DestroyActor` (`self.PillarRef`))))
      (`self.K2_SetActorLocation` _bossref (`self.BossStartLocation`) false false)
      (`CharacterMovementComponent.SetMovementMode` (`Character.CharacterMovement` (`self.BossRef`)) "MOVE_Walking" 0)
      (set `/Game/Blueprints/BP_Boss.IsBusy` false _bossref)
      (`self.K2_DestroyActor`))))

(fn `UserConstructionScript`)