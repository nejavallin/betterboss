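; BP_Ability_ExpandingRing is an ability actor that spawns a ring which grows over time and then removes itself.
; On BeginPlay it prints a debug message and plays ExpansionTimeline, whose ScaleMultiplier track uniformly drives the world scale of RingCollision.
; The actor destroys itself when the timeline finishes.
; The graph has no active overlap handling, so it applies no effect to actors the ring touches.
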(event `self.ReceiveBeginPlay`
  (`KismetSystemLibrary.PrintString` "EXPANDING RING SPAWNED!")
  (bind (_direction _scalemultiplier) (`Timeline|ExpansionTimeline`)
    (:`Update`
      (`SceneComponent.SetWorldScale3D` (`self.RingCollision`) (`KismetMathLibrary.MakeVector` _scalemultiplier _scalemultiplier _scalemultiplier)))
    (:`Finished`
      (`self.K2_DestroyActor`))))

(fn `UserConstructionScript`
  (`parent.UserConstructionScript`))