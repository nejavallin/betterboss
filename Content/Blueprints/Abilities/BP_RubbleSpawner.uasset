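; Arena hazard spawner that, when the player first overlaps its trigger, starts a looping rubble timer and wakes an inactive BP_Enemy_BiggerGuy.
; Each tick of the timer runs repeated randomized line traces around the arena center, then spawns three BP_Ability_RubbleZone actors just above the last impact point.
; The safe-radius and spawn-spacing checks are disconnected, so HasOverlap never blocks a spawn.
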(event `self.Trigger.OnComponentBeginOverlap`
  (params (OverlappedComponent :type "PrimitiveComponent Object Reference") (OtherActor :type "Actor Object Reference") (OtherComp :type "PrimitiveComponent Object Reference") (OtherBodyIndex :type Integer) (bFromSweep :type Boolean) (SweepResult :type "HitResult Structure (by ref)"))
  (cast `/Game/Blueprints/Player/BP_PlayerChar` OtherActor)
  (`PrimitiveComponent.SetCollisionEnabled` (`self.Trigger`) "NoCollision")
  (`KismetSystemLibrary.K2_SetTimerDelegate` (delegate `SpawnRubble`) (`self.SpawnInterval`) true)
  ; Toggles the first BiggerGuy in the level if hes inactive
  (bind _returnvalue (`GameplayStatics.GetActorOfClass` "/Game/Blueprints/AI/BP_Enemy_BiggerGuy.BP_Enemy_BiggerGuy_C"))
  (if (not (`/Game/Blueprints/AI/BP_Enemy_BiggerGuy.ActiveOnSpawn` _returnvalue))
    (`/Game/Blueprints/AI/BP_Enemy_BiggerGuy.RepossesSelf` _returnvalue)))

(event `SpawnRubble`
  (bind _returnvalue (`KismetMathLibrary.RandomFloatInRange` 0.0 360.0))
  (bind _returnvalue_2 (`KismetMathLibrary.RandomFloatInRange` 0.0 (`self.ArenaRadius`)))
  (bind _z (.z (`self.ArenaCenter`)))
  (bind _returnvalue_3 (+ (.x (`self.ArenaCenter`)) (* (`KismetMathLibrary.DegCos` _returnvalue) _returnvalue_2)))
  (bind _returnvalue_4 (+ (.y (`self.ArenaCenter`)) (* (`KismetMathLibrary.DegSin` _returnvalue) _returnvalue_2)))
  (for _ (range 1 (+ (`self.MaxRetries`) 1))
    (set `self.HasOverlap` false)
    (bind _outhit (`KismetSystemLibrary.LineTraceSingle` (`KismetMathLibrary.MakeVector` _returnvalue_3 _returnvalue_4 (+ _z 500.0)) (`KismetMathLibrary.MakeVector` _returnvalue_3 _returnvalue_4 (- _z 450.0)) "TraceTypeQuery1"))
    (if true
      (`GameplayStatics.GetActorOfClass` "/Game/Blueprints/BP_Boss.BP_Boss_C")
      (bind _returnvalue_5 (`GameplayStatics.GetActorOfClass` "/Game/Env_SciFi/Blueprints/BP_Orb_Red.BP_Orb_Red_C"))))
  (if (not (`self.HasOverlap`))
    (for _ (range 1 4)
      (`|SpawnActorFromClass` "/Game/Blueprints/Abilities/RubbleBoulderRingCombo/BP_Ability_RubbleZone.BP_Ability_RubbleZone_C" (`KismetMathLibrary.MakeTransform` (`KismetMathLibrary.MakeVector` (.x (`.ImpactPoint` (`GameplayStatics.BreakHitResult` _outhit))) (.y (`.ImpactPoint` (`GameplayStatics.BreakHitResult` _outhit))) (+ (.z (`.ImpactPoint` (`GameplayStatics.BreakHitResult` _outhit))) 110.0))) "Undefined" "MultiplyWithRoot" null null))))

(fn `UserConstructionScript`)