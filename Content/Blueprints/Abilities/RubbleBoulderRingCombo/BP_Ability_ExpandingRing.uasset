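; Expanding shockwave ring ability actor that damages the player once as it grows outward, then destroys itself.
; On BeginPlay a timeline scales the flat ring mesh horizontally over its lifetime.
; Each update it hit-tests player character 0 mathematically, using a 2D distance band behind the ring edge plus a height tolerance, then applies damage through the player's health component.
; The mesh overlap event is left empty, its damage logic disconnected.
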(event `self.ReceiveBeginPlay`
  (bind _returnvalue (`self.K2_GetActorLocation`))
  (bind _returnvalue_2 (`GameplayStatics.GetPlayerCharacter` 0))
  (bind _returnvalue_3 (`self.K2_GetActorLocation` _returnvalue_2))
  (bind _returnvalue_4 (`KismetMathLibrary.Distance2D` (`KismetMathLibrary.Conv_VectorToVector2D` _returnvalue) (`KismetMathLibrary.Conv_VectorToVector2D` _returnvalue_3)))
  (set `self.HasDamagedPlayer` false)
  (`KismetSystemLibrary.PrintString` "EXPANDING RING SPAWNED!")
  (bind (_direction _scalemultiplier) (`Timeline|ExpansionTimeline`)
    (:`Update`
      (`SceneComponent.SetWorldScale3D` (`self.VisualRing`) (`KismetMathLibrary.MakeVector` _scalemultiplier _scalemultiplier 0.5))
      (if (not (`self.HasDamagedPlayer`))
        (bind _returnvalue_5 (* _scalemultiplier 70.0))
        (if (and (and (<= _returnvalue_4 _returnvalue_5) (>= _returnvalue_4 (- _returnvalue_5 150.0))) (< (`KismetMathLibrary.Abs` (- (.z _returnvalue) (.z _returnvalue_3))) 100.0))
          (set `self.HasDamagedPlayer` true)
          (bind _asbp_player_char (cast `/Game/Blueprints/Player/BP_PlayerChar` _returnvalue_2))
          (`/Game/Blueprints/BPC_Health.ApplyDamage` (`/Game/Blueprints/Player/BP_PlayerChar.BPC_Health` _asbp_player_char) 5.0))))
    (:`Finished`
      (`self.K2_DestroyActor`))))

(event `self.VisualRing.OnComponentBeginOverlap`
  (params (OverlappedComponent :type "PrimitiveComponent Object Reference") (OtherActor :type "Actor Object Reference") (OtherComp :type "PrimitiveComponent Object Reference") (OtherBodyIndex :type Integer) (bFromSweep :type Boolean) (SweepResult :type "HitResult Structure (by ref)")))

(fn `UserConstructionScript`
  (`parent.UserConstructionScript`))