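; Rubble zone ability actor that slows players inside it, then spawns a gravity ball.
; Capsule overlap cuts player walk speed to 30% of a cached original, updated only above a speed threshold, and restores it on exit.
; After a ten-second delay it spawns BP_Ability_GravityBall high above itself and destroys itself.
; EndPlay restores speed through OverlappedPlayer, but both overlap handlers only clear that reference.
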(event `self.ReceiveBeginPlay`
  (`KismetSystemLibrary.Delay` 10.0)
  (`|SpawnActorFromClass` "/Game/Blueprints/Abilities/RubbleBoulderRingCombo/BP_Ability_GravityBall.BP_Ability_GravityBall_C" (`KismetMathLibrary.MakeTransform` (+ (`self.K2_GetActorLocation`) (0.0 0.0 1500.0))) "Undefined" "MultiplyWithRoot" null null)
  (`self.K2_DestroyActor`))

(event `self.Capsule.OnComponentBeginOverlap`
  (params (OverlappedComponent :type "PrimitiveComponent Object Reference") (OtherActor :type "Actor Object Reference") (OtherComp :type "PrimitiveComponent Object Reference") (OtherBodyIndex :type Integer) (bFromSweep :type Boolean) (SweepResult :type "HitResult Structure (by ref)"))
  (bind _asbp_player_char (cast `/Game/Blueprints/Player/BP_PlayerChar` OtherActor))
  (set `self.OverlappedPlayer` null)
  (bind _charactermovement (`Character.CharacterMovement` _asbp_player_char))
  (bind _maxwalkspeed (`CharacterMovementComponent.MaxWalkSpeed` _charactermovement))
  (if (> _maxwalkspeed 400.0)
    (set `self.OriginalWalkSpeed` _maxwalkspeed))
  (set `CharacterMovementComponent.MaxWalkSpeed` (* (`self.OriginalWalkSpeed`) 0.3) _charactermovement))

(event `self.Capsule.OnComponentEndOverlap`
  (params (OverlappedComponent :type "PrimitiveComponent Object Reference") (OtherActor :type "Actor Object Reference") (OtherComp :type "PrimitiveComponent Object Reference") (OtherBodyIndex :type Integer))
  (bind _asbp_player_char (cast `/Game/Blueprints/Player/BP_PlayerChar` OtherActor))
  (set `CharacterMovementComponent.MaxWalkSpeed` (`self.OriginalWalkSpeed`) (`Character.CharacterMovement` _asbp_player_char))
  (set `self.OverlappedPlayer` null))

(event `self.ReceiveEndPlay`
  (params (EndPlayReason :type "EEndPlayReason Enum" :default "Destroyed"))
  (`/Engine/EditorBlueprintResources/StandardMacros.IsValid` (`self.OverlappedPlayer`)
    (:`Is Valid`
      (set `CharacterMovementComponent.MaxWalkSpeed` (`self.OriginalWalkSpeed`) (`Character.CharacterMovement` (`self.OverlappedPlayer`))))))

(fn `UserConstructionScript`)