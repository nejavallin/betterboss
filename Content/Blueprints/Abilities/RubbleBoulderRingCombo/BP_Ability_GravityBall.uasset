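; BP_Ability_GravityBall is a ball ability actor in the RubbleBoulderRingCombo set that damages the player and turns into an expanding ring on impact.
; On BeginPlay, its sphere is set to ignore every BP_TestEnemy when moving.
; Overlapping BP_PlayerChar applies heavy damage through its health component without destroying the ball.
; A blocking hit spawns BP_Ability_ExpandingRing at the impact point, then destroys the ball.
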(event `self.Sphere.OnComponentHit`
  (params (HitComponent :type "PrimitiveComponent Object Reference") (OtherActor :type "Actor Object Reference") (OtherComp :type "PrimitiveComponent Object Reference") (NormalImpulse :type "Vector Structure") (Hit :type "HitResult Structure (by ref)"))
  (`|SpawnActorFromClass` "/Game/Blueprints/Abilities/RubbleBoulderRingCombo/BP_Ability_ExpandingRing.BP_Ability_ExpandingRing_C" (`KismetMathLibrary.MakeTransform` (`.ImpactPoint` (`GameplayStatics.BreakHitResult` Hit))) "AlwaysSpawn" "MultiplyWithRoot" null null)
  (`self.K2_DestroyActor`))

(event `self.ReceiveBeginPlay`
  (bind _outactors (`GameplayStatics.GetAllActorsOfClass` "/Game/Blueprints/AI/BP_TestEnemy.BP_TestEnemy_C"))
  (for _array_element _outactors
    (`PrimitiveComponent.IgnoreActorWhenMoving` (`self.Sphere`) _array_element true)))

(event `self.Sphere.OnComponentBeginOverlap`
  (params (OverlappedComponent :type "PrimitiveComponent Object Reference") (OtherActor :type "Actor Object Reference") (OtherComp :type "PrimitiveComponent Object Reference") (OtherBodyIndex :type Integer) (bFromSweep :type Boolean) (SweepResult :type "HitResult Structure (by ref)"))
  (bind _asbp_player_char (cast `/Game/Blueprints/Player/BP_PlayerChar` OtherActor))
  (`/Game/Blueprints/BPC_Health.ApplyDamage` (`/Game/Blueprints/Player/BP_PlayerChar.BPC_Health` _asbp_player_char) 90.0)
  (`KismetSystemLibrary.PrintString` "BALL HIT"))

(fn `UserConstructionScript`
  (`parent.UserConstructionScript`))