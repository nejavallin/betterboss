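; Boss ability actor that calls three successive artillery strikes on the player's position, keeping the boss marked busy until it finishes and destroys itself.
; On spawn it reads damage, timings, debug draw and telegraph VFX from the boss's ability data table.
; Each strike locks a ground-level point under the player, shows the telegraph, then spawns lightning and sphere-traces to damage a hit actor's health component.
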(event `self.ReceiveBeginPlay`
  (bind (_value _foundability) (`/Game/Blueprints/BP_Boss.GetDTAbility` (`self.BossRef`) "NewEnumerator1"))
  (bind (_abilityid _damage _minrange _maxrange _cooldown _validphases _usecount _currentuses _telegraphduration _useduration _debug _ns_vfx) (break `/Game/Blueprints/F_AbiltyStruct` _value))
  (if _foundability
    (set `self.Damage` _damage)
    (set `self.TelegraphDuration` _telegraphduration)
    (set `self.Duration` _useduration)
    (set `self.Draw Debug Type` _debug)
    (set `self.TelegraphVFX` _ns_vfx))
  (set `/Game/Blueprints/BP_Boss.IsBusy` true (`self.BossRef`))
  (set `self.CurrentStrike` 1)
  (`self.DoStrike`))

(event `DoStrike`
  (bind _output_get (set `self.StrikeLocation` (`KismetMathLibrary.MakeVector` (.x (`self.K2_GetActorLocation` (`/Game/Blueprints/BP_Boss.PlayerRef` (`self.BossRef`)))) (.y (`self.K2_GetActorLocation` (`/Game/Blueprints/BP_Boss.PlayerRef` (`self.BossRef`)))) (- (.z (`self.K2_GetActorLocation` (`/Game/Blueprints/BP_Boss.PlayerRef` (`self.BossRef`)))) 85.0))))
  (bind _returnvalue (`NiagaraFunctionLibrary.SpawnSystemAtLocation` (`self.TelegraphVFX`) _output_get))
  (set `self.TelegraphVFXRef` _returnvalue)
  (`KismetSystemLibrary.Delay` (`self.TelegraphDuration`))
  (`ActorComponent.K2_DestroyComponent` (`self.TelegraphVFXRef`))
  (`NiagaraFunctionLibrary.SpawnSystemAtLocation` "/Game/__LightningThunderVFX/NS/NS_Lightning_Single.NS_Lightning_Single" (`self.StrikeLocation`) (struct) (5.0 5.0 5.0))
  (bind _outhit (`KismetSystemLibrary.SphereTraceSingleForObjects` :`Start` (`self.StrikeLocation`) :`End` (+ (`self.StrikeLocation`) (0.0 0.0 10.0)) :`Radius` 150.0 :`ObjectTypes` (`|MakeArray` "ObjectTypeQuery3" "ObjectTypeQuery2" :!type "EObjectTypeQuery Enum") :`DrawDebugType` (`self.Draw Debug Type`)))
  (bind (_bblockinghit _binitialoverlap _time _distance _location _impactpoint _normal _impactnormal _physmat _hitactor) (`GameplayStatics.BreakHitResult` _outhit))
  (bind _returnvalue_2 (`self.GetComponentByClass` _hitactor "/Game/Blueprints/BPC_Health.BPC_Health_C"))
  ; Add Validity Check to fix runtime compliation error
  (if (and (`KismetSystemLibrary.IsValid` _hitactor) (`KismetSystemLibrary.IsValid` _returnvalue_2))
    (`/Game/Blueprints/BPC_Health.ApplyDamage` _returnvalue_2 (`self.Damage`)))
  (`KismetSystemLibrary.Delay` (`self.Duration`))
  (`/Engine/EditorBlueprintResources/StandardMacros.IncrementInt` (`self.CurrentStrike`)
    (:`  `
      (if (<= (`self.CurrentStrike`) 3)
        (`self.DoStrike`)
        (else
          (set `/Game/Blueprints/BP_Boss.IsBusy` false (`self.BossRef`))
          (`self.K2_DestroyActor`))))))

(fn `UserConstructionScript`)