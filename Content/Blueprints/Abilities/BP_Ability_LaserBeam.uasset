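; Boss laser beam ability actor that damages the player when its Beam component begins overlapping them.
; A WorldStatic line trace from the actor to the player checks for cover, and damage lands only if nothing blocks it.
; Damage and trace debug drawing come from the boss's ability data table entry, with a default damage fallback if the entry is not found.
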(event `self.ReceiveBeginPlay`)

(event `self.Beam.OnComponentBeginOverlap`
  (params (OverlappedComponent :type "PrimitiveComponent Object Reference") (OtherActor :type "Actor Object Reference") (OtherComp :type "PrimitiveComponent Object Reference") (OtherBodyIndex :type Integer) (bFromSweep :type Boolean) (SweepResult :type "HitResult Structure (by ref)"))
  (bind (_value _foundability) (`/Game/Blueprints/BP_Boss.GetDTAbility` (`self.BossRef`) "NewEnumerator0"))
  (bind _asbp_player_char (cast `/Game/Blueprints/Player/BP_PlayerChar` OtherActor))
  (bind _outhit (`KismetSystemLibrary.LineTraceSingleForObjects` (`self.K2_GetActorLocation`) (`self.K2_GetActorLocation` _asbp_player_char) (`|MakeArray` "ObjectTypeQuery1" :!type "EObjectTypeQuery Enum") false (`|MakeArray` self :!type "Actor Object Reference") (`.Debug_42_EAB8721F494F727CC721EB92E7F822FD` (break `/Game/Blueprints/F_AbiltyStruct` _value))))
  (if (not (`GameplayStatics.BreakHitResult` _outhit))
    (`/Game/Blueprints/Components/BPC_Health.ApplyDamage` (`/Game/Blueprints/Player/BP_PlayerChar.BPC_Health` _asbp_player_char) (`KismetMathLibrary.SelectFloat` (`.Damage_39_C7BFA74E404A3AFC605FC09B79B9FDF1` (break `/Game/Blueprints/F_AbiltyStruct` _value)) (`self.DefaultDaamge`) _foundability))
    (`KismetSystemLibrary.PrintString` "BEAM HIT")))

(fn `UserConstructionScript`)