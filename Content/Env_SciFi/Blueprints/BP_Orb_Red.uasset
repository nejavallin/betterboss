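; BP_Orb_Red is a damageable orb with an on-screen health bar that gives way to the boss when it dies.
; BPC_Health updates the bar, while the collider ignores BP_Enemy_BiggerGuy actors during movement.
; ApplyDamage cancels the player's dash and launches them away.
; On death, a delayed loop over those enemies destroys them, plays an impact effect, repeats the knockback, spawns BP_Boss and destroys the orb.
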(event `UpdateOrbHealthBar`
  (params (NewHealth :type "Float (double-precision) (by ref)"))
  (bind _bpc_health (`self.BPC_Health`))
  ; HealthBar
  (`/Game/UI/WBP_OrbHealthBar.Orb Update Health Percent` (`self.OrbHealthBar`) (/ (`/Game/Blueprints/BPC_Health.Health` _bpc_health) (`/Game/Blueprints/BPC_Health.MaxHealth` _bpc_health))))

(event `self.ReceiveBeginPlay`
  (`|ExecutionSequence`
    (:`then_0`
      (bind _outactors (`GameplayStatics.GetAllActorsOfClass` "/Game/Blueprints/AI/BP_Enemy_BiggerGuy.BP_Enemy_BiggerGuy_C"))
      (for _array_element _outactors
        (`PrimitiveComponent.IgnoreActorWhenMoving` (`self.SphereCollider`) _array_element true)))
    (:`then_1`
      ; HealthBar
      (bind _returnvalue (`|CreateWidget` "/Game/UI/WBP_OrbHealthBar.WBP_OrbHealthBar_C" (`GameplayStatics.GetPlayerController` 0)))
      (bind _output_get (set `self.OrbHealthBar` _returnvalue))
      (`UserWidget.AddToViewport` _output_get 0)
      (add `/Game/Blueprints/BPC_Health.OnHealthUpdated` (`self.BPC_Health`) (delegate `UpdateOrbHealthBar`)))))

(event `self.BPC_Health.OnDeath`
  (bind _returnvalue (`GameplayStatics.GetPlayerCharacter` 0))
  (`KismetSystemLibrary.Delay` 1.0)
  (`Widget.RemoveFromParent` (`self.OrbHealthBar`))
  (bind _outactors (`GameplayStatics.GetAllActorsOfClass` "/Game/Blueprints/AI/BP_Enemy_BiggerGuy.BP_Enemy_BiggerGuy_C"))
  (for _array_element _outactors
    (`self.K2_DestroyActor` _array_element)
    (`NiagaraFunctionLibrary.SpawnSystemAtLocation` "/Game/VFX/Mixed_Magic_VFX_Pack/VFX/Sperate_VFX/NS_Magma_Shot_Impact.NS_Magma_Shot_Impact" (`self.K2_GetActorLocation`))
    (bind _asbp_player_char (cast `/Game/Blueprints/Player/BP_PlayerChar` _returnvalue))
    (set `/Game/Blueprints/Player/BP_PlayerChar.Is Dashing` false _asbp_player_char)
    (`TimelineComponent.Stop` (`/Game/Blueprints/Player/BP_PlayerChar.Timeline` _asbp_player_char))
    (bind _charactermovement (`Character.CharacterMovement` (`CharacterMovementComponent.GetCharacterOwner` (`Character.CharacterMovement` _asbp_player_char))))
    (`ActorComponent.Activate` _charactermovement false)
    (`CharacterMovementComponent.SetMovementMode` _charactermovement "MOVE_Falling" 0)
    (`Character.StopAnimMontage` _asbp_player_char null)
    (`Character.LaunchCharacter` _asbp_player_char (* (`KismetMathLibrary.Normal` (`KismetMathLibrary.MakeVector` (.x (`KismetMathLibrary.Normal` (- (`self.K2_GetActorLocation` _returnvalue) (`self.K2_GetActorLocation`)))) (.y (`KismetMathLibrary.Normal` (- (`self.K2_GetActorLocation` _returnvalue) (`self.K2_GetActorLocation`)))) 0.5)) (3000.0 3000.0 3000.0)) false false)
    (`KismetSystemLibrary.Delay` 0.1)
    (`|SpawnActorFromClass` "/Game/Blueprints/BP_Boss.BP_Boss_C" (`self.GetTransform`) "AlwaysSpawn" "MultiplyWithRoot" null null)
    (`self.K2_DestroyActor`)))

(event `/Game/Blueprints/Interfaces/BPI_Damageable.Apply Damage`
  (params (Damage :type "Float (double-precision)") (`Damage Causer` :type "Actor Object Reference") (`Damage Location` :type "Vector Structure") (`Damage Impulse` :type "Vector Structure"))
  ; Knockback when player punch
  (bind _asbp_player_char (cast `/Game/Blueprints/Player/BP_PlayerChar` (`GameplayStatics.GetPlayerCharacter` 0)))
  (set `/Game/Blueprints/Player/BP_PlayerChar.Is Dashing` false _asbp_player_char)
  (`TimelineComponent.Stop` (`/Game/Blueprints/Player/BP_PlayerChar.Timeline` _asbp_player_char))
  (bind _charactermovement (`Character.CharacterMovement` (`CharacterMovementComponent.GetCharacterOwner` (`Character.CharacterMovement` _asbp_player_char))))
  (`ActorComponent.Activate` _charactermovement false)
  (`CharacterMovementComponent.SetMovementMode` _charactermovement "MOVE_Falling" 0)
  (`Character.StopAnimMontage` _asbp_player_char null)
  (`Character.LaunchCharacter` _asbp_player_char (* (`KismetMathLibrary.Normal` (`KismetMathLibrary.MakeVector` (.x (`KismetMathLibrary.Normal` (- (`self.K2_GetActorLocation` _asbp_player_char) (`self.K2_GetActorLocation`)))) (.y (`KismetMathLibrary.Normal` (- (`self.K2_GetActorLocation` _asbp_player_char) (`self.K2_GetActorLocation`)))) 0.5)) (4000.0 4000.0 50.0)) false false))

(fn `UserConstructionScript`)